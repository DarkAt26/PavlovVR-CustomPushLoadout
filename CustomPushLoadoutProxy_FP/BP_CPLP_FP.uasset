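; Custom Push loadout proxy that equips a pawn and sets its skin when a loadout slot is taken, with two example classes as templates.
; OnLoadoutTaken caches the pawn, switches on the slot to call helper functions, then returns false.
; Helpers spawn items and weapons with attachments through the game logic, and grant ammo and skins through the player proxy.
; Unwired copies of the helper nodes sit in the graph as a palette.
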(fn `Give Ammo`
  (params (`Ammo Type` :type "/Game/CustomPushLoadoutProxy_FP/AmmoTypes_Enum Enum" :default "NewEnumerator0") (Amount :type Integer))
  (`Pavlov_PlayerProxy.AddAmmo` (`Pavlov_Library.GetPlayerProxy` (`self.F_Pawn`)) (`KismetStringLibrary.Conv_StringToName` (`|GetEnumeratorNameAsString` `Ammo Type`)) Amount))

(fn `OnLoadoutTaken`
  (params (LoadoutSlot :type Name) (Pawn :type "Pawn Object Reference"))
  (returns (SpawnTransform :type "Transform Structure") (ReturnValue :type Boolean))
  (set `self.F_Pawn` Pawn)
  (`|ExecutionSequence`
    (:`then_0`
      (switch `name` LoadoutSlot
        (:`ExampleClass1`
          ;[1 1 1] ExampleClass1
          (`self.Spawn Weapon With Attachments` "ar" true false 0 true true (`|MakeArray` "reddot" "supp_rifle" "Grip_Angled" :!type "Name"))
          (`self.Spawn Item / Weapon` "PushBomb" false true 5 false false)
          (`self.Spawn Item / Weapon` "antitankmine" false true 6 false false)
          (`self.Give Ammo` "NewEnumerator1" 400)
          (`self.Set Player Skin` "cop"))
        (:`ExampleClass2`
          ;[1 1 1] ExampleClass2
          (`self.Spawn Item / Weapon` "cet9")
          (`self.Set Player Skin` "prisoner"))))
    (:`then_1`
      (return (struct) false))))

(fn `Set Player Skin`
  (params (Id :type Name))
  (`Pavlov_PlayerProxy.SetPlayerSkin` (`Pavlov_Library.GetPlayerProxy` (`self.F_Pawn`)) Id))

(fn `Spawn Item / Weapon`
  (params (Id :type Name) (`Dominant Hand` :type Boolean :default true) (`Spawn In Inventory` :type Boolean) (`Inventory Slot` :type Integer) (`Spawn With Magazine` :type Boolean :default true) (`Spawn With Default Attachments` :type Boolean :default true))
  (`Pavlov_GameLogic.SpawnItem` (`Pavlov_Library.GetGameLogic`) (make `PavlovItemSpawnParams` Id (`Pawn.PlayerState` (`self.F_Pawn`)) `Dominant Hand` `Spawn In Inventory` `Inventory Slot` false (struct) `Spawn With Magazine` `Spawn With Default Attachments`)))

(fn `Spawn Weapon With Attachments`
  (params (Id :type Name) (`Dominant Hand` :type Boolean :default true) (`Spawn In Inventory` :type Boolean) (`Inventory Slot` :type Integer) (`Spawn With Magazine` :type Boolean :default true) (`Spawn With Default Attachments` :type Boolean :default true) (Attachments :type "Array of Name"))
  (bind _returnvalue (`Pavlov_Library.GetGameLogic`))
  (bind (_bsuccessful _item) (`Pavlov_GameLogic.SpawnItemWRef` _returnvalue (make `PavlovItemSpawnParams` Id (`Pawn.PlayerState` (`self.F_Pawn`)) `Dominant Hand` `Spawn In Inventory` `Inventory Slot` false (struct) `Spawn With Magazine` `Spawn With Default Attachments`)))
  (`Pavlov_GameLogic.SpawnAttachments` _returnvalue (make `PavlovAttachmentSpawnParams` Attachments _item)))

(fn `UserConstructionScript`)