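; Template actor for customizing Push mode loadout rooms and classes, with placeholder class logic and helpers for items, ammo and skins.
; Construction positions both team rooms and sets optional replacement room child actors.
; After startup delays, collision overlaps find rooms and lockers by display name, hide replaced rooms, and pass locker parts, read by child index, to a stubbed customization function.
; The loadout-taken delegate spawns gear per class.
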(event `CustomEvent_0`
  (bind _returnvalue (`self.GetComponentByClass` (`self.PushLoadoutRoom_Defender`) "/Script/Engine.StaticMeshComponent"))
  (bind _returnvalue_2 (`self.GetComponentByClass` (`self.PushLoadoutRoom_Attacker`) "/Script/Engine.StaticMeshComponent"))
  (`KismetSystemLibrary.Delay` 0.2)
  (`|ExecutionSequence`
    (:`then_0`
      (`|ExecutionSequence`
        (:`then_0`
          (`KismetArrayLibrary.Array_Append` (`self.PushLoadoutRoom_Actors`) (`PrimitiveComponent.GetOverlappingActors` (`self.Collision_Defender`) null))
          (`KismetArrayLibrary.Array_Append` (`self.PushLoadoutRoom_Actors`) (`PrimitiveComponent.GetOverlappingActors` (`self.Collision_Attacker`) null)))
        (:`then_1`
          (for _array_element (`self.PushLoadoutRoom_Actors`)
            (`|ExecutionSequence`
              (:`then_0`
                (bind _returnvalue_3 (`KismetSystemLibrary.GetDisplayName` _array_element))
                (if (`KismetStringLibrary.Contains` _returnvalue_3 "BP_PushLootLocker_C")
                  (`KismetArrayLibrary.Array_Add` (`self.PushLoadoutRoom_Lockers`) _array_element)))
              (:`then_1`
                (if (`KismetStringLibrary.Contains` _returnvalue_3 "BP_PushLoadoutRoom_Defender_C")
                  (set `self.PushLoadoutRoom_Defender` _array_element)))
              (:`then_2`
                (if (`KismetStringLibrary.Contains` _returnvalue_3 "BP_PushLoadoutRoom_Attacker_C")
                  (set `self.PushLoadoutRoom_Attacker` _array_element))))))
        (:`then_2`
          (`ActorComponent.K2_DestroyComponent` (`self.Collision_Defender`))
          (`ActorComponent.K2_DestroyComponent` (`self.Collision_Attacker`)))))
    (:`then_1`
      (for _array_element_2 (`self.PushLoadoutRoom_Lockers`)
        (bind _astext_render_component (cast `TextRenderComponent` (`SceneComponent.GetChildComponent` (`Actor.RootComponent` _array_element_2) 10) :!pure true))
        (`self.Custom Locker Code` (`KismetStringLibrary.Conv_StringToName` (`KismetStringLibrary.Split` (`KismetTextLibrary.Conv_TextToString` (`TextRenderComponent.Text` _astext_render_component)) " - ")) _array_element_2 (`Actor.RootComponent` _array_element_2) (`self.GetComponentByClass` _array_element_2 "/Script/Engine.SkeletalMeshComponent") (cast `StaticMeshComponent` (`SceneComponent.GetChildComponent` (`Actor.RootComponent` _array_element_2) 9) :!pure true) _astext_render_component (cast `StaticMeshComponent` (`SceneComponent.GetChildComponent` (`Actor.RootComponent` _array_element_2) 11) :!pure true) (cast `SkeletalMeshComponent` (`SceneComponent.GetChildComponent` (`Actor.RootComponent` _array_element_2) 0) :!pure true) (cast `SkeletalMeshComponent` (`SceneComponent.GetChildComponent` (`Actor.RootComponent` _array_element_2) 1) :!pure true) (cast `SkeletalMeshComponent` (`SceneComponent.GetChildComponent` (`Actor.RootComponent` _array_element_2) 2) :!pure true) (cast `SkeletalMeshComponent` (`SceneComponent.GetChildComponent` (`Actor.RootComponent` _array_element_2) 3) :!pure true) (cast `SkeletalMeshComponent` (`SceneComponent.GetChildComponent` (`Actor.RootComponent` _array_element_2) 4) :!pure true) (cast `SkeletalMeshComponent` (`SceneComponent.GetChildComponent` (`Actor.RootComponent` _array_element_2) 5) :!pure true) (cast `SkeletalMeshComponent` (`SceneComponent.GetChildComponent` (`Actor.RootComponent` _array_element_2) 6) :!pure true) (cast `SkeletalMeshComponent` (`SceneComponent.GetChildComponent` (`Actor.RootComponent` _array_element_2) 7) :!pure true))))
    (:`then_2`
      (`|ExecutionSequence`
        (:`then_0`
          (`/Engine/EditorBlueprintResources/StandardMacros.IsValid` (`self.CustomLoadoutRoom_Defender`)
            (:`Is Valid`
              (`SceneComponent.SetVisibility` _returnvalue false false)
              (`PrimitiveComponent.SetCollisionEnabled` _returnvalue "NoCollision"))))
        (:`then_1`
          (`/Engine/EditorBlueprintResources/StandardMacros.IsValid` (`self.CustomLoadoutRoom_Attacker`)
            (:`Is Valid`
              (`SceneComponent.SetVisibility` _returnvalue_2 false false)
              (`PrimitiveComponent.SetCollisionEnabled` _returnvalue_2 "NoCollision"))))))))

(event `self.ReceiveBeginPlay`
  (`KismetSystemLibrary.Delay` 1.0)
  (add `/Game/CPP/BP_CPP_Call.OnPushLoadoutTaken` (`self.PushLoadoutProxy`) (delegate `OnPushLoadoutTaken`))
  (`|ExecutionSequence`
    (:`then_0`
      (`KismetSystemLibrary.Delay` 4.0)
      (`self.CustomEvent_0`))))

(event `OnPushLoadoutTaken`
  (params (`Loadout Class` :type Name) (Pawn :type "Pawn Object Reference"))
  (set `self.F_Pawn` Pawn)
  (switch `name` `Loadout Class`
    (:`Class1`
      (`self.Spawn Item / Weapon` "ar"))))

(fn `Add Item SK`
  (params (RelativeTransform :type "Transform Structure") (Item :type "SkeletalMesh Object Reference") (AttachTo :type "SceneComponent Object Reference"))
  (`/Engine/EditorBlueprintResources/StandardMacros.IsValid` Item
    (:`Is Valid`
      (bind _returnvalue (`AddComponent|NODE_AddSkeletalMeshComponent-3` :`RelativeTransform` RelativeTransform))
      (`SkinnedMeshComponent.SetSkinnedAssetAndUpdate` _returnvalue Item true)
      (`SceneComponent.K2_AttachToComponent` _returnvalue AttachTo "None" "KeepRelative" "KeepRelative" "KeepRelative" true))))

(fn `Add Item SM`
  (params (RelativeTransform :type "Transform Structure") (Item :type "StaticMesh Object Reference") (AttachTo :type "SceneComponent Object Reference"))
  (`/Engine/EditorBlueprintResources/StandardMacros.IsValid` Item
    (:`Is Valid`
      (bind _returnvalue (`AddComponent|NODE_AddStaticMeshComponent-6` :`RelativeTransform` RelativeTransform))
      (`StaticMeshComponent.SetStaticMesh` _returnvalue Item)
      (`SceneComponent.K2_AttachToComponent` _returnvalue AttachTo "None" "KeepRelative" "KeepRelative" "KeepRelative" true))))

(fn `Add Weapon`
  (params (AttachTo :type "SceneComponent Object Reference") (`Transfrom (Relative)` :type "Transform Structure") (Weapon :type "SkeletalMesh Object Reference") (Magazine :type "StaticMesh Object Reference") (Scope :type "StaticMesh Object Reference") (Grip :type "StaticMesh Object Reference") (Attachment :type "StaticMesh Object Reference") (Suppressor :type "StaticMesh Object Reference"))
  (`/Engine/EditorBlueprintResources/StandardMacros.IsValid` Weapon
    (:`Is Valid`
      (bind _returnvalue (`AddComponent|NODE_AddSkeletalMeshComponent-2` :`RelativeTransform` `Transfrom (Relative)`))
      (`SkinnedMeshComponent.SetSkinnedAssetAndUpdate` _returnvalue Weapon true)
      (`SceneComponent.K2_AttachToComponent` _returnvalue AttachTo "None" "KeepRelative" "KeepRelative" "KeepRelative" true)
      (for _array_element (`|MakeArray` "Magazine" "Picatinny" "Grip" "Accessory" "Suppressor" :!type "Name")
        (bind _value (`BlueprintMapLibrary.Map_Find` (`|MakeMap` "Magazine" Magazine "Picatinny" Scope "Grip" Grip "Accessory" Attachment "Suppressor" Suppressor :!type "Name") _array_element))
        (`/Engine/EditorBlueprintResources/StandardMacros.IsValid` _value
          (:`Is Valid`
            (bind _returnvalue_2 (`AddComponent|NODE_AddStaticMeshComponent-5`))
            (`StaticMeshComponent.SetStaticMesh` _returnvalue_2 _value)
            (`SceneComponent.K2_AttachToComponent` _returnvalue_2 _returnvalue _array_element "KeepRelative" "KeepRelative" "KeepRelative" true)))))))

(fn `Custom Locker Code`
  (params (`Class Name` :type Name) (`Locker Actor` :type "Actor Object Reference") (`Locker Actor Root` :type "SceneComponent Object Reference") (`Locker Mesh` :type "SkeletalMeshComponent Object Reference") (`Shelf Mesh` :type "StaticMeshComponent Object Reference") (TextRender :type "TextRenderComponent Object Reference") (`TextRender Background Mesh` :type "StaticMeshComponent Object Reference") (`PrimaryHandWeapon Mesh` :type "SkeletalMeshComponent Object Reference") (`PrimaryBack Mesh` :type "SkeletalMeshComponent Object Reference") (`Secondary Mesh` :type "SkeletalMeshComponent Object Reference") (`Knife Mesh` :type "SkeletalMeshComponent Object Reference") (`Meds Mesh` :type "SkeletalMeshComponent Object Reference") (`Syringe Mesh` :type "SkeletalMeshComponent Object Reference") (`Mine Mesh` :type "SkeletalMeshComponent Object Reference") (`Bomb Mesh` :type "SkeletalMeshComponent Object Reference"))
  ;[1 1 1] LockerClasses Stuff
  (switch `name` `Class Name`))

(fn `Give Ammo`
  (params (AmmoType :type "/Game/CPP/AmmoTypes_Enum Enum" :default "NewEnumerator0") (Amount :type Integer))
  (`Pavlov_PlayerProxy.AddAmmo` (`Pavlov_Library.GetPlayerProxy` (`self.F_Pawn`)) (`KismetStringLibrary.Conv_StringToName` (`|GetEnumeratorNameAsString` AmmoType)) Amount))

(fn `Set Player Skin`
  (params (Id :type Name))
  (`Pavlov_PlayerProxy.SetPlayerSkin` (`Pavlov_Library.GetPlayerProxy` (`self.F_Pawn`)) Id))

(fn `Spawn Item / Weapon`
  (params (Id :type Name) (`Dominant Hand` :type Boolean :default true) (`Spawn In Inventory` :type Boolean) (`Inventory Slot` :type Integer) (`Spawn With Magazine` :type Boolean :default true) (`Spawn With Default Attachments` :type Boolean :default true))
  (`Pavlov_GameLogic.SpawnItem` (`Pavlov_Library.GetGameLogic`) (make `PavlovItemSpawnParams` Id (`Pawn.PlayerState` (`self.F_Pawn`)) `Dominant Hand` `Spawn In Inventory` `Inventory Slot` false (struct) `Spawn With Magazine` `Spawn With Default Attachments`)))

(fn `Spawn Weapon With Attachments`
  (params (`Params Id` :type Name) (`Params Dominant Hand` :type Boolean :default true) (`Params Spawn In Inventory` :type Boolean) (`Params Inventory Slot` :type Integer) (`Params Spawn With Magazine` :type Boolean :default true) (`Params Spawn With Default Attachments` :type Boolean :default true) (InputPin :type "Array of Name"))
  (bind _returnvalue (`Pavlov_Library.GetGameLogic`))
  (bind (_bsuccessful _item) (`Pavlov_GameLogic.SpawnItemWRef` _returnvalue (make `PavlovItemSpawnParams` `Params Id` (`Pawn.PlayerState` (`self.F_Pawn`)) `Params Dominant Hand` `Params Spawn In Inventory` `Params Inventory Slot` false (struct) `Params Spawn With Magazine` `Params Spawn With Default Attachments`)))
  (`Pavlov_GameLogic.SpawnAttachments` _returnvalue (make `PavlovAttachmentSpawnParams` InputPin _item)))

(fn `UserConstructionScript`
  (bind _pushsettings (`self.PushSettings`))
  (bind _loadoutroom_defender (`self.LoadoutRoom_Defender`))
  (bind _customloadoutroom_defender (`self.CustomLoadoutRoom_Defender`))
  (bind _loadoutroom_attacker (`self.LoadoutRoom_Attacker`))
  (bind _customloadoutroom_attacker (`self.CustomLoadoutRoom_Attacker`))
  (bind (_defenderloadoutlocation_boverrideloadoutlocation _defenderloadoutlocation_loadoutspawnlocation) (break `PushLoadoutLocation` (`Pavlov_PushSettings.DefenderLoadoutLocation` _pushsettings)))
  (bind (_attackerloadoutlocation_boverrideloadoutlocation _attackerloadoutlocation_loadoutspawnlocation) (break `PushLoadoutLocation` (`Pavlov_PushSettings.AttackerLoadoutLocation` _pushsettings)))
  (`|ExecutionSequence`
    (:`then_0`
      (`|ExecutionSequence`
        (:`then_0`
          (`|ExecutionSequence`
            (:`then_0`
              (`SceneComponent.K2_SetWorldTransform` (`self.Attacker`) (`KismetMathLibrary.MakeTransform` (+ _attackerloadoutlocation_loadoutspawnlocation (-600.0 -300.0 0.0))) false false))
            (:`then_1`
              (`SceneComponent.K2_SetWorldTransform` (`self.Defender`) (`KismetMathLibrary.MakeTransform` (+ _defenderloadoutlocation_loadoutspawnlocation (-600.0 -300.0 0.0))) false false))))
        (:`then_1`
          (`|ExecutionSequence`
            (:`then_0`
              (if (`KismetSystemLibrary.IsValidClass` _loadoutroom_defender)
                (`ChildActorComponent.SetChildActorClass` _customloadoutroom_defender _loadoutroom_defender)
                (else
                  (`ActorComponent.K2_DestroyComponent` _customloadoutroom_defender))))
            (:`then_1`
              (if (`KismetSystemLibrary.IsValidClass` _loadoutroom_attacker)
                (`ChildActorComponent.SetChildActorClass` _customloadoutroom_attacker _loadoutroom_attacker)
                (else
                  (`ActorComponent.K2_DestroyComponent` _customloadoutroom_attacker))))))))))